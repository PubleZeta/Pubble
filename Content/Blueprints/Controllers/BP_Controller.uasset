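; BP_Controller is a player controller that drives a BP_Pad pawn sideways and views it through a separate camera actor.
; On BeginPlay it casts the controlled pawn to BP_Pad and blends the view to the BP_Camera found in the level.
; The LateralMovement axis moves the pad along its right vector, remapped through a sign-preserving response curve and scaled by an input multiplier.
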(event `self.ReceiveBeginPlay`
  (bind _asbp_pad (cast `/Game/Blueprints/Pawns/BP_Pad` (`self.K2_GetPawn`)))
  (set `self.Pad` _asbp_pad)
  (bind _returnvalue (`GameplayStatics.GetActorOfClass` "/Game/Blueprints/Actors/BP_Camera.BP_Camera_C"))
  (bind _output_get (set `self.SemiTopDownCamera` _returnvalue))
  (`self.SetViewTargetWithBlend` _output_get))

(event `InputAxis|LateralMovement`
  (params (AxisValue :type "Float (single-precision)"))
  (bind _pad (`self.Pad`))
  (`Pawn.AddMovementInput` _pad (`self.GetActorRightVector` _pad) (* (`self.GetInputMapped` AxisValue) (`self.InputMultiplier`)) false))

(fn `GetInputMapped`
  (params (Input :type "Float (double-precision)"))
  (returns (ReturnValue :type "Float (double-precision)"))
  (locals (Sign :type "Float (double-precision)" :default 0.0))
  (if (< Input 0.0)
    (set `local.Sign` -1.0)
    (else
      (set `local.Sign` 1.0)))
  (return (* (`CurveFloat.GetFloatValue` (`self.InputCurve`) (`KismetMathLibrary.Abs` Input)) (`local.Sign`))))

(fn `UserConstructionScript`)