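; Movement component for BP_Ball that keeps the physics-simulated ball travelling at a constant speed.
; On BeginPlay it launches the mesh along its forward vector with a velocity-change impulse, then after a short delay clamps velocity magnitude to Speed every tick.
; Increasespeed multiplies Speed by a factor.
; Helper functions cover per-frame speed, vector angles and sign operations, while InitializeVelocity duplicates the launch but is not wired in.
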(event `self.ReceiveBeginPlay`
  ;[1 1 1] get ball reference add initial impulse
  (bind _asbp_ball (cast `/Game/Blueprints/Actors/BP_Ball` (`self.GetOwner`)))
  (bind _output_get (set `self.CurrentBall` _asbp_ball))
  (`PrimitiveComponent.AddImpulse` (`/Game/Blueprints/Actors/BP_Ball.StaticMesh` (`self.CurrentBall`)) (* (`SceneComponent.GetForwardVector` (`/Game/Blueprints/Actors/BP_Ball.StaticMesh` _output_get)) (`self.Speed`)) "None" true)
  (`KismetSystemLibrary.Delay` 0.2)
  (set `self.gamestarted` true))

(event `self.ReceiveTick`
  (params (DeltaSeconds :type "Float (single-precision)"))
  (set `self.DeltaSec` DeltaSeconds)
  (if (`self.gamestarted`)
    (`self.Clamp Velocity`)))

(event `Clamp Velocity`
  (bind _speed (`self.Speed`))
  (`PrimitiveComponent.SetPhysicsLinearVelocity` (`/Game/Blueprints/Actors/BP_Ball.StaticMesh` (`self.CurrentBall`)) (`KismetMathLibrary.ClampVectorSize` (`Actor.GetVelocity` (`self.CurrentBall`)) _speed _speed) false "None"))

(event `Increase speed`
  (set `self.Speed` (* (`self.Speed`) (`self.Speed Increase Factor`))))

(fn `GetAngleBetweenTwoVectors`
  (params (Vector1 :type "Vector Structure") (Vector2 :type "Vector Structure"))
  (returns (Angle :type "Float (double-precision)") (axis :type "Vector Structure"))
  (bind _returnvalue (`KismetMathLibrary.Normal` Vector2))
  (bind _returnvalue_2 (`KismetMathLibrary.Normal` Vector1))
  (return (`KismetMathLibrary.Abs` (`KismetMathLibrary.DegAcos` (`KismetMathLibrary.Dot_VectorVector` _returnvalue_2 _returnvalue))) (`KismetMathLibrary.Cross_VectorVector` _returnvalue_2 _returnvalue)))

(fn `GetBallSpeed`
  (returns (ReturnValue :type "Float (double-precision)"))
  (return (* (`self.Speed`) (`self.DeltaSec`))))

(fn `GetFloatSign`
  (params (FloatValue :type "Float (double-precision)"))
  (returns (FloatPositive :type Boolean))
  (locals (sfsdfsf :type Boolean))
  (if (>= FloatValue 0.0)
    (set `local.sfsdfsf` true)
    (else
      (set `local.sfsdfsf` false)))
  (return (`local.sfsdfsf`)))

(fn `InitializeVelocity`
  (bind _asbp_ball (cast `/Game/Blueprints/Actors/BP_Ball` (`self.GetOwner`)))
  (bind _output_get (set `self.CurrentBall` _asbp_ball))
  (`PrimitiveComponent.AddImpulse` (`/Game/Blueprints/Actors/BP_Ball.StaticMesh` (`self.CurrentBall`)) (* (`SceneComponent.GetForwardVector` (`/Game/Blueprints/Actors/BP_Ball.StaticMesh` _output_get)) (`self.Speed`)) "None" true)
  (set `self.gamestarted` true))

(fn `InvertSignVectorComponent`
  (params (VectorComponent :type "/Game/Blueprints/Enum/Enum_VectorComponents Enum" :default "NewEnumerator0") (Vector :type "Vector Structure"))
  (returns (InvertedVector :type "Vector Structure"))
  (locals (Vec :type "Vector Structure"))
  (bind (_vec_x _vec_y _vec_z) (`KismetMathLibrary.BreakVector` (`local.Vec`)))
  (bind (_vec_x_2 _vec_y_2 _vec_z_2) (`KismetMathLibrary.BreakVector` (`local.Vec`)))
  (bind (_vec_x_3 _vec_y_3 _vec_z_3) (`KismetMathLibrary.BreakVector` (`local.Vec`)))
  (set `local.Vec` Vector)
  (switch `/Game/Blueprints/Enum/Enum_VectorComponents` VectorComponent
    (:`NewEnumerator0`
      (set `local.Vec` (`KismetMathLibrary.MakeVector` (* _vec_x_2 -1.0) _vec_y_2 _vec_z_2)))
    (:`NewEnumerator1`
      (set `local.Vec` (`KismetMathLibrary.MakeVector` _vec_x_3 (* _vec_y_3 -1.0) _vec_z_3)))
    (:`NewEnumerator2`
      (set `local.Vec` (`KismetMathLibrary.MakeVector` _vec_x _vec_y (* _vec_z -1.0)))))
  (return (`local.Vec`)))

(fn `SameSign?`
  (params (Vec :type "Vector Structure") (Vec2 :type "Vector Structure"))
  (returns (x :type Boolean) (y :type Boolean))
  (return (and (`self.GetFloatSign` (.x Vec)) (`self.GetFloatSign` (.x Vec2))) (and (`self.GetFloatSign` (.y Vec)) (`self.GetFloatSign` (.y Vec2)))))