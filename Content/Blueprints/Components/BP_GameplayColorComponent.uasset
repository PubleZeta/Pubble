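; Actor component that gives its owner a gameplay color, applied to a static mesh material and an optional point light.
; Initialize creates a dynamic instance of the prototype color material and caches the owner's light.
; Setters pick either a random color or one no BP_Obstacle currently uses, optionally firing a color-change event.
; The current color is read back from the material as an enum, and emissive strength is adjustable.
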(event `self.ReceiveBeginPlay`)

(event `Initialize`
  (bind _returnvalue (`self.GetOwner`))
  (bind _returnvalue_2 (`Actor.GetComponentByClass` _returnvalue "/Script/Engine.StaticMeshComponent"))
  (bind _returnvalue_3 (`Actor.GetComponentByClass` _returnvalue "/Script/Engine.PointLightComponent"))
  (`/Engine/EditorBlueprintResources/StandardMacros.IsValid` _returnvalue_2
    (:`Is Valid`
      (bind _output_get (set `self.StaticMesh` _returnvalue_2))
      (bind _returnvalue_4 (`PrimitiveComponent.CreateDynamicMaterialInstance` _output_get 0 "/Game/Blueprints/Materials/Masters/MM_ColorPrototypeMaterial.MM_ColorPrototypeMaterial" "None"))
      (set `self.DynamicMaterial` _returnvalue_4)
      (`/Engine/EditorBlueprintResources/StandardMacros.IsValid` _returnvalue_3
        (:`Is Valid`
          (set `self.PointLight` _returnvalue_3))))))

(fn `GetCurrentColor`
  (returns (ColorEnum :type "/Game/Blueprints/Enum/Enum_Colors Enum"))
  (bind _returnvalue (`MaterialInstanceDynamic.K2_GetVectorParameterValue` (`self.DynamicMaterial`) "Color"))
  (return (`/Game/Blueprints/Libraries/BPL_GamePlayColors.GetEnumByLinearColor` _returnvalue)))

(fn `SetAvailableColor`
  (params (`CallOnColorChangeEvent?` :type Boolean :default true))
  (locals (AllColors :type "Array of /Game/Blueprints/Enum/Enum_Colors Enum") (CallEvent :type Boolean :default false))
  (bind _allcolors (`local.AllColors`))
  (set `local.CallEvent` `CallOnColorChangeEvent?`)
  (bind _outactors (`GameplayStatics.GetAllActorsOfClass` "/Game/Blueprints/Actors/BP_Obstacle.BP_Obstacle_C"))
  (for _array_element _outactors
    (bind _colorenum (`self.GetCurrentColor` (`/Game/Blueprints/Actors/BP_Obstacle.BP_GameplayColorComponent` _array_element)))
    (if (`KismetArrayLibrary.Array_Contains` (`local.AllColors`) _colorenum)
      (`KismetArrayLibrary.Array_RemoveItem` (`local.AllColors`) _colorenum)))
  (if (!= (`KismetArrayLibrary.Array_Length` _allcolors) 0)
    (`self.SetComponentsColor` (`/Game/Blueprints/Libraries/BPL_GamePlayColors.GetLinearColorByEnum` (`|GetArrayItem` _allcolors (`KismetMathLibrary.RandomIntegerInRange` 0 (`KismetArrayLibrary.Array_LastIndex` _allcolors)))) (`local.CallEvent`))
    (else
      (`KismetSystemLibrary.PrintString` "No available colors")))
  (return))

(fn `SetComponentsColor`
  (params (Color :type "LinearColor Structure") (`CallOnColorChangeEvent?` :type Boolean :default true))
  (bind _pointlight (`self.PointLight`))
  (`MaterialInstanceDynamic.SetVectorParameterValue` (`self.DynamicMaterial`) "Color" Color)
  (`/Engine/EditorBlueprintResources/StandardMacros.IsValid` _pointlight
    (:`Is Valid`
      (`LightComponent.SetLightColor` _pointlight Color true))
    (:`Is Not Valid`
      _))
  (if `CallOnColorChangeEvent?`
    (`self.OnColorChange`)))

(fn `SetEmissiveMultiplier`
  (params (Value :type "Float (double-precision)"))
  (`MaterialInstanceDynamic.SetScalarParameterValue` (`self.DynamicMaterial`) "EmissiveMultiplier" Value))

(fn `SetRandomColor`
  (params (`CallOnColorChangeEvent?` :type Boolean :default true))
  (locals (Color :type "Array of /Game/Blueprints/Enum/Enum_Colors Enum"))
  (bind _color (`local.Color`))
  (`self.SetComponentsColor` (`/Game/Blueprints/Libraries/BPL_GamePlayColors.GetLinearColorByEnum` (`|GetArrayItem` _color (`KismetMathLibrary.RandomIntegerInRange` 0 (`KismetArrayLibrary.Array_LastIndex` _color)))) `CallOnColorChangeEvent?`))