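; BP_Ball is the color-coded ball that scores points by hitting actors of its own color.
; It waits for its color component's dynamic material, then picks red or blue and binds a color-match event that increases the game mode's score.
; Each hit on a new actor either fires that event or, for mismatched obstacles, recolors both and speeds up the ball.
; Color changes trigger a timeline-driven emissive flash.
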(event `self.ReceiveBeginPlay`
  (bind _bp_gameplaycolorcomponent (`self.BP_GameplayColorComponent`))
  (`/Game/Blueprints/Components/BP_GameplayColorComponent.Initialize` _bp_gameplaycolorcomponent)
  (`/Engine/EditorBlueprintResources/StandardMacros.IsValid` (`/Game/Blueprints/Components/BP_GameplayColorComponent.DynamicMaterial` _bp_gameplaycolorcomponent) :!label _label
    (:`Is Valid`
      (`/Game/Blueprints/Components/BP_GameplayColorComponent.SetRandomColorRedOrBlue` (`self.BP_GameplayColorComponent`) true)
      (add `self.Colormatching` (delegate `Color Matching`)))
    (:`Is Not Valid`
      (`KismetSystemLibrary.Delay` 0.2)
      (goto _label))))

(event `Color Matching`
  (bind _asbp_pubble_game_mode (cast `/Game/Blueprints/GameModes/BP_Pubble_GameMode` (`GameplayStatics.GetGameMode`)))
  (`/Game/Blueprints/GameModes/BP_Pubble_GameMode.Increase Score` _asbp_pubble_game_mode))

(event `self.StaticMesh.OnComponentHit`
  (params (HitComponent :type "PrimitiveComponent Object Reference") (OtherActor :type "Actor Object Reference") (OtherComp :type "PrimitiveComponent Object Reference") (NormalImpulse :type "Vector Structure") (Hit :type "HitResult Structure (by ref)"))
  (bind _lasthitactor (`self.LastHitActor`))
  (bind _returnvalue (`self.GetComponentByClass` (`self.LastHitActor`) "/Game/Blueprints/Components/BP_GameplayColorComponent.BP_GameplayColorComponent_C"))
  (`/Engine/EditorBlueprintResources/StandardMacros.IsValid` _lasthitactor
    (:`Is Valid`
      (if (!= _lasthitactor OtherActor)
        (set `self.LastHitActor` OtherActor :!label _label_2)
        (`/Engine/EditorBlueprintResources/StandardMacros.IsValid` _returnvalue
          (:`Is Valid`
            (if (`|EnumEquality` (`/Game/Blueprints/Components/BP_GameplayColorComponent.GetCurrentColor` _returnvalue) (`/Game/Blueprints/Components/BP_GameplayColorComponent.GetCurrentColor` (`self.BP_GameplayColorComponent`)))
              (`KismetSystemLibrary.PrintString` "Same color")
              (`self.Colormatching`)
              (else
                (bind _asbp_obstacle (cast `/Game/Blueprints/Actors/BP_Obstacle` (`self.LastHitActor`)))
                (`/Game/Blueprints/Components/BP_GameplayColorComponent.SetAvailableColor` (`/Game/Blueprints/Actors/BP_Obstacle.BP_GameplayColorComponent` _asbp_obstacle) true)
                (`/Game/Blueprints/Components/BP_BallMovementComponent.Increase speed` (`self.BP_BallMovementComponent`))
                (`/Game/Blueprints/Components/BP_GameplayColorComponent.SetRandomColor` (`self.BP_GameplayColorComponent`) true)
                (`KismetSystemLibrary.PrintString` "Change Color")))))))
    (:`Is Not Valid`
      (goto _label_2))))

(event `self.BP_GameplayColorComponent.OnColorChange`
  (if (not (`TimelineComponent.IsPlaying` (`self.EmissiveTimeline`)))
    (bind (_direction _emissivecurve) (`Timeline|EmissiveTimeline` :!via `PlayFromStart`)
      (:`Update`
        (`/Game/Blueprints/Components/BP_GameplayColorComponent.SetEmissiveMultiplier` (`self.BP_GameplayColorComponent`) (`KismetMathLibrary.Lerp` 2.0 150.0 _emissivecurve))))))

(fn `UserConstructionScript`)