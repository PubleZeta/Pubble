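; Blueprint function library that converts between a gameplay color enum (red, blue, green, yellow, invalid) and linear colors.
; GetDefaultsGameplayColor supplies the shared palette for both lookups, with the invalid value mapping to opaque black.
; Reverse lookup uses exact RGBA equality without tolerance, so any unmatched color returns the invalid value.
; A helper writes an enum's color to a named material vector parameter, given a static mesh.
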(fn `GetDefaultsGameplayColor`
  (returns (Red :type "LinearColor Structure") (Green :type "LinearColor Structure") (Blue :type "LinearColor Structure") (Yellow :type "LinearColor Structure"))
  (locals (Red_Loc :type "LinearColor Structure" :default (struct :`R` 1.0 :`A` 1.0)) (Green_Loc :type "LinearColor Structure" :default (struct :`G` 1.0 :`A` 1.0)) (Blue_Loc :type "LinearColor Structure" :default (struct :`B` 1.0 :`A` 1.0)) (Yellow_Loc :type "LinearColor Structure" :default (struct :`R` 1.0 :`G` 1.0 :`A` 1.0)))
  (return (`local.Red_Loc`) (`local.Green_Loc`) (`local.Blue_Loc`) (`local.Yellow_Loc`)))

(fn `GetEnumByLinearColor`
  (params (Color :type "LinearColor Structure"))
  (returns (`Enum Color` :type "/Game/Blueprints/Enum/Enum_Colors Enum"))
  (locals (red :type "LinearColor Structure") (blue :type "LinearColor Structure") (green :type "LinearColor Structure") (yellow :type "LinearColor Structure") (`input color` :type "LinearColor Structure") (enumOutput :type "/Game/Blueprints/Enum/Enum_Colors Enum" :default "NewEnumerator0"))
  (bind (_red _green _blue _yellow) (`self.GetDefaultsGameplayColor` null))
  (set `local.input color` Color)
  (bind _samecolor_ (`self.SameColor?` (`local.input color`) _red))
  (if _samecolor_
    (set `local.enumOutput` "NewEnumerator0")
    (else
      (bind _samecolor__2 (`self.SameColor?` (`local.input color`) _green))
      (if _samecolor__2
        (set `local.enumOutput` "NewEnumerator2")
        (else
          (bind _samecolor__3 (`self.SameColor?` (`local.input color`) _blue))
          (if _samecolor__3
            (set `local.enumOutput` "NewEnumerator1")
            (else
              (bind _samecolor__4 (`self.SameColor?` (`local.input color`) _yellow))
              (if _samecolor__4
                (set `local.enumOutput` "NewEnumerator3")
                (else
                  (set `local.enumOutput` "NewEnumerator4")))))))))
  (return (`local.enumOutput`)))

(fn `GetLinearColorByEnum`
  (params (EnumColor :type "/Game/Blueprints/Enum/Enum_Colors Enum" :default "NewEnumerator0"))
  (returns (Color :type "LinearColor Structure"))
  (locals (NewLocalVar_0 :type "Float (double-precision)") (Color_Loc :type "LinearColor Structure" :default (struct :`A` 1.0)))
  (bind (_red _green _blue _yellow) (`self.GetDefaultsGameplayColor` null))
  (bind _output_get (set `local.Color_Loc` (select `/Game/Blueprints/Enum/Enum_Colors` EnumColor :`NewEnumerator0` _red :`NewEnumerator1` _blue :`NewEnumerator2` _green :`NewEnumerator3` _yellow)))
  (return _output_get))

(fn `SameColor?`
  (params (Color1 :type "LinearColor Structure") (Color2 :type "LinearColor Structure"))
  (returns (`SameColor?` :type Boolean))
  (bind (_r _g _b _a) (break `LinearColor` Color1))
  (bind (_r_2 _g_2 _b_2 _a_2) (break `LinearColor` Color2))
  (return (and (== _r _r_2) (== _g _g_2) (== _b _b_2) (== _a _a_2))))

(fn `Set Material Color by Enum`
  (params (`Enum_ Color` :type "/Game/Blueprints/Enum/Enum_Colors Enum (by ref)") (StaticMesh :type "StaticMesh Object Reference (by ref)") (ParameterName :type "Name (by ref)"))
  (`KismetMaterialLibrary.SetVectorParameterValue` StaticMesh null ParameterName (`self.GetLinearColorByEnum` `Enum_ Color`))
  (return))